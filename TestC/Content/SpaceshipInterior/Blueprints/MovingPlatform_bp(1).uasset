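; Moving platform actor that slides a cube mesh from its placed position to the position of a Box component when play begins.
; BeginPlay caches both world locations and sets the PlatformMovement timeline's play rate to the inverse of the Sekunden (seconds) variable to control travel time.
; Each timeline update lerps the cube between the two points without sweeping.
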(event EventBeginPlay
  (Components|Timeline|SetPlayRate (Variables|Default|GetPlatformMovement) (/ 1.0 (Variables|Default|GetSekunden)))
  (Variables|Default|SetStartOrt (Transformation|GetWorldLocation (Variables|Default|GetCube)))
  (Variables|Default|SetEndOrt (Transformation|GetWorldLocation (Variables|Default|GetBox)))
  (bind _newtrack_0 (Timeline|PlatformMovement Play)
    (:Update
      (Transformation|SetWorldLocation (Variables|Default|GetCube) (Math|Vector|Lerp(Vector) (Variables|Default|GetStartOrt) (Variables|Default|GetEndOrt) _newtrack_0) false false))))

(fn ConstructionScript)