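; Kabel is a cable pickup actor in the spaceship interior that the player collects with E.
; Its Box overlap with the ThirdPersonCharacter shows an InteractionBp prompt and enables input; leaving reverses both.
; Pressing E marks the prompt as pressed, waits briefly, then destroys the actor and calls Kabel0.
; Kabel0 prints a debug message and sets PickedUpKabel on the referenced Halterung.
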(event OnComponentBeginOverlap(Box)
  (params (OverlappedComponent :type Primitive%20Component%20Object%20Reference) (OtherActor :type Actor%20Object%20Reference) (OtherComp :type Primitive%20Component%20Object%20Reference) (OtherBodyIndex :type Integer) (bFromSweep :type Boolean) (SweepResult :type Hit%20Result%20Structure%20%28by%20ref%29))
  (Utilities|Casting|CastToThirdPersonCharacter OtherActor)
  (bind _returnvalue (UserInterface|CreateWidget "/Game/Dessert/InteractionBp.InteractionBp_C"))
  (UserInterface|Viewport|AddtoViewport _returnvalue 0)
  (Input|EnableInput (Game|GetPlayerController 0)))

(event OnComponentEndOverlap(Box)
  (params (OverlappedComponent :type Primitive%20Component%20Object%20Reference) (OtherActor :type Actor%20Object%20Reference) (OtherComp :type Primitive%20Component%20Object%20Reference) (OtherBodyIndex :type Integer))
  (Utilities|Casting|CastToThirdPersonCharacter OtherActor)
  (Widget|RemovefromParent (stale OnComponentBeginOverlap(Box) _returnvalue))
  (Input|DisableInput (Game|GetPlayerController 0)))

(event Custom|Kabel0
  (Development|PrintString "kabel" true true "(R=0.385322,G=0.713542,B=0.014510,A=1.000000)")
  (bind _ashalterung (Utilities|Casting|CastToHalterung (Variables|Default|GetHalterung)))
  (Variables|/Game/SpaceshipInterior/Blueprints/Halterung.Halterung_C|SetPickedUpKabel _ashalterung true))

(event EventBeginPlay)

(event Collision|EventActorBeginOverlap
  (params (OtherActor :type Actor%20Object%20Reference)))

(event EventTick
  (params (DeltaSeconds :type Float%20%28single-precision%29)))

(event Input|KeyboardEvents|E
  (params (Key :type Key%20Structure :default "None"))
  (:Pressed
    (Variables|/Game/Dessert/InteractionBp.InteractionBp_C|SetIsPressed (stale OnComponentBeginOverlap(Box) _returnvalue) true)
    (Utilities|FlowControl|Delay 0.2)
    (Variables|/Game/Dessert/InteractionBp.InteractionBp_C|SetIsPressed (stale OnComponentBeginOverlap(Box) _returnvalue) true)
    (Actor|DestroyActor)
    (CallFunction|Kabel0)))

(fn ConstructionScript)