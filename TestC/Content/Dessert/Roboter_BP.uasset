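; Robot Blueprint that continuously follows the player's ThirdPersonCharacter.
; BeginPlay caches the character reference and starts FollowChar, a self-calling loop that issues AI MoveTo and repeats after a short delay.
; A distance check would switch the move target to the robot itself, but its zero threshold means it always chases the player.
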(event Custom|FollowChar
  (if (>= (Transformation|GetDistanceTo (Variables|Default|GetChar%20Ref)) 0.0)
    (AI|AIMoveTo 0 "0, 0, 0" (Variables|Default|GetChar%20Ref) 5.0 false
      (:then
        _))
    (else
      (AI|AIMoveTo 0 "0, 0, 0" self 5.0 false
        (:then
          _))))
  (Utilities|FlowControl|Delay 0.2)
  (CallFunction|FollowChar))

(event EventBeginPlay
  (bind _asthird_person_character (Utilities|Casting|CastToThirdPersonCharacter (Game|GetPlayerCharacter 0)))
  (Variables|Default|SetChar%20Ref _asthird_person_character)
  (CallFunction|FollowChar))

(fn ConstructionScript)