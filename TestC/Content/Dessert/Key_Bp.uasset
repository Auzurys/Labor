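; Key pickup actor in the Dessert folder that the third-person character collects with the E key.
; Overlapping its box shows an interaction widget and enables input on the actor; leaving removes both.
; Pressing E flags the widget as pressed, waits briefly, hides the key meshes and disables collision.
; It then sets its own HaveKey flag and prints a pickup message.
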(event OnComponentBeginOverlap(Box)
  (params (OverlappedComponent :type Primitive%20Component%20Object%20Reference) (OtherActor :type Actor%20Object%20Reference) (OtherComp :type Primitive%20Component%20Object%20Reference) (OtherBodyIndex :type Integer) (bFromSweep :type Boolean) (SweepResult :type Hit%20Result%20Structure%20%28by%20ref%29))
  (Utilities|Casting|CastToThirdPersonCharacter OtherActor)
  (bind _returnvalue (UserInterface|CreateWidget "/Game/Dessert/InteractionBp.InteractionBp_C"))
  (UserInterface|Viewport|AddtoViewport _returnvalue 0)
  (Input|EnableInput (Game|GetPlayerController 0)))

(event OnComponentEndOverlap(Box)
  (params (OverlappedComponent :type Primitive%20Component%20Object%20Reference) (OtherActor :type Actor%20Object%20Reference) (OtherComp :type Primitive%20Component%20Object%20Reference) (OtherBodyIndex :type Integer))
  (Utilities|Casting|CastToThirdPersonCharacter OtherActor)
  (Widget|RemovefromParent (stale OnComponentBeginOverlap(Box) _returnvalue))
  (Input|DisableInput (Game|GetPlayerController 0)))

(event Custom|Add%20Key
  (Variables|Default|Sethave%20key true)
  (Development|PrintString "Key aquired"))

(event Input|KeyboardEvents|E
  (params (Key :type Key%20Structure :default "None"))
  (:Pressed
    (Variables|/Game/Dessert/InteractionBp.InteractionBp_C|SetIsPressed (stale OnComponentBeginOverlap(Box) _returnvalue) true)
    (Utilities|FlowControl|Delay 0.2)
    (Variables|/Game/Dessert/InteractionBp.InteractionBp_C|SetIsPressed (stale OnComponentBeginOverlap(Box) _returnvalue) true)
    (Rendering|SetVisibility (Variables|Default|GetKey_Cylinder) false false)
    (Collision|SetCollisionEnabled (Variables|Default|GetBox) "NoCollision")
    (CallFunction|AddKey)))

(fn ConstructionScript)