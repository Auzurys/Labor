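; Checkpoint actor that saves its own location when the third-person character enters its trigger box.
; On overlap it prints a debug message, then loads the StefanieSGO save in slot "1" or creates one if none exists.
; It writes its root component's world location into SavedLoc and saves back to that slot, so each touched checkpoint overwrites the previous position.
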(event OnComponentBeginOverlap(Box)
  (params (OverlappedComponent :type Primitive%20Component%20Object%20Reference) (OtherActor :type Actor%20Object%20Reference) (OtherComp :type Primitive%20Component%20Object%20Reference) (OtherBodyIndex :type Integer) (bFromSweep :type Boolean) (SweepResult :type Hit%20Result%20Structure%20%28by%20ref%29))
  (Utilities|Casting|CastToThirdPersonCharacter OtherActor)
  (Development|PrintString "Checkpoint reached!")
  (bind _returnvalue (SaveGame|DoesSaveGameExist "1"))
  (if _returnvalue
    (bind _returnvalue_2 (SaveGame|LoadGamefromSlot "1"))
    (bind _asstefanie_sgo (Utilities|Casting|CastToStefanieSGO _returnvalue_2))
    (Variables|/Game/Teststuff/StefanieSGO.StefanieSGO_C|SetSaved_Loc _asstefanie_sgo (Transformation|GetWorldLocation (Variables|Default|GetDefaultSceneRoot)))
    (SaveGame|SaveGametoSlot _asstefanie_sgo "1")
    (else
      (bind _returnvalue_3 (SaveGame|CreateSaveGameObject "/Game/Teststuff/StefanieSGO.StefanieSGO_C"))
      (Variables|/Game/Teststuff/StefanieSGO.StefanieSGO_C|SetSaved_Loc _returnvalue_3 (Transformation|GetWorldLocation (Variables|Default|GetDefaultSceneRoot)))
      (SaveGame|SaveGametoSlot _returnvalue_3 "1"))))

(event EventBeginPlay)

(event Collision|EventActorBeginOverlap
  (params (OtherActor :type Actor%20Object%20Reference)))

(event EventTick
  (params (DeltaSeconds :type Float%20%28single-precision%29)))

(fn ConstructionScript)