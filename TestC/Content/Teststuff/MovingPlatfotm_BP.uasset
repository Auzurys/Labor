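; A test moving platform Blueprint that slides its Cube component from its starting position to the position of a Box marker component.
; On BeginPlay it caches both world locations as start and end points.
; It then plays the PlatformMovement timeline at a rate of one over Sekunden, lerping the Cube between them without sweep.
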(event EventBeginPlay
  (Components|Timeline|SetPlayRate (Variables|Default|GetPlatformMovement) (/ 1.0 (Variables|Default|GetSekunden)))
  (Variables|Default|SetStartort (Transformation|GetWorldLocation (Variables|Default|GetCube)))
  (Variables|Default|SetEndort (Transformation|GetWorldLocation (Variables|Default|GetBox)))
  (bind _newtrack_0 (Timeline|PlatformMovement Play)
    (:Update
      (Transformation|SetWorldLocation (Variables|Default|GetCube) (Math|Vector|Lerp(Vector) (Variables|Default|GetStartort) (Variables|Default|GetEndort) _newtrack_0) false false))))

(fn ConstructionScript)