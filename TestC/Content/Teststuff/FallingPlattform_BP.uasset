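; Falling platform actor that drops shortly after something overlaps its trigger box, then returns to its starting spot.
; BeginPlay stores the Cube's world transform as the reset point.
; A Box overlap passes a DoOnce gate, waits briefly, then enables physics simulation on the Cube.
; After a further delay it disables physics, snaps the Cube back without sweep and resets the gate for reuse.
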(event OnComponentBeginOverlap(Box)
  (params (OverlappedComponent :type Primitive%20Component%20Object%20Reference) (OtherActor :type Actor%20Object%20Reference) (OtherComp :type Primitive%20Component%20Object%20Reference) (OtherBodyIndex :type Integer) (bFromSweep :type Boolean) (SweepResult :type Hit%20Result%20Structure%20%28by%20ref%29))
  (Utilities|FlowControl|DoOnce false :!label _label
    (:Completed
      (Utilities|FlowControl|Delay 1.0)
      (Physics|SetSimulatePhysics (Variables|Default|GetCube) true)
      (Utilities|FlowControl|Delay 4.0)
      (Physics|SetSimulatePhysics (Variables|Default|GetCube) false)
      (Transformation|SetWorldTransform (Variables|Default|GetCube) (Variables|Default|GetOriginal%20Location) false false)
      (goto _label Reset))))

(event EventBeginPlay
  (Variables|Default|SetOriginal%20Location (Transformation|GetWorldTransform (Variables|Default|GetCube))))

(event Collision|EventActorBeginOverlap
  (params (OtherActor :type Actor%20Object%20Reference)))

(event EventTick
  (params (DeltaSeconds :type Float%20%28single-precision%29)))

(fn ConstructionScript)